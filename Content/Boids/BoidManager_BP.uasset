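; Boid manager actor that spawns a flock of Boid_BP actors inside a box volume.
; The construction script caches the origin, scaled extent and rotation of the BoidContainer box from the actor.
; On BeginPlay it spawns the configured number of boids at random points and rotations, passing each the bounds and a reference to itself.
; The random spawn point ignores the box rotation, which is only handed to the boids.
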(event EventBeginPlay
  (for _index (range 1 (Variables|Default|GetBoids))
    (Game|SpawnActorfromClass "/Game/Boids/Boid_BP.Boid_BP_C" (Math|Transform|MakeTransform (Math|Random|RandomPointinBoundingBox (Variables|Default|GetBoxOrigin) (Variables|Default|GetBoxExtent)) (Math|Random|RandomRotator false)) "Undefined" 0 (Variables|Default|GetBoxOrigin) (Variables|Default|GetBoxExtent) (Variables|Default|GetBoxRotation) self)))

(fn ConstructionScript
  (Variables|Default|SetBoxOrigin (Transformation|GetActorLocation))
  (Variables|Default|SetBoxExtent (Components|Box|GetScaledBoxExtent (Variables|Default|GetBoidContainer)))
  (Variables|Default|SetBoxRotation (Transformation|GetActorRotation)))