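; Test player controller that lets the player spawn Boid_BP actors where they aim.
; Each tick it traces from the focal location along the control rotation, ignoring all existing boids and drawing a debug line, then stores the impact point nudged along the surface normal as Target.
; Left mouse click spawns a randomly rotated boid at Target, without checking whether the trace hit anything.
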(event EventTick
  (params (DeltaSeconds :type Float%20%28single-precision%29))
  (bind _returnvalue (Class|PlayerController|GetFocalLocation))
  (bind _outactors (Actor|GetAllActorsOfClass "/Game/Boids/Boid_BP.Boid_BP_C"))
  (bind _outhit (Collision|LineTraceByChannel _returnvalue (+ _returnvalue (* (Math|Vector|GetForwardVector (Pawn|GetControlRotation :!class /Script/Engine.Controller)) 5000)) "TraceTypeQuery1" false _outactors "ForOneFrame"))
  (Variables|Default|SetTarget (+ (.ImpactPoint (Collision|BreakHitResult _outhit)) (* (.ImpactNormal (Collision|BreakHitResult _outhit)) 20))))

(event EventBeginPlay)

(event Input|MouseEvents|LeftMouseButton
  (params (Key :type Key%20Structure :default "AnyKey"))
  (:Pressed
    (Game|SpawnActorfromClass "/Game/Boids/Boid_BP.Boid_BP_C" (Math|Transform|MakeTransform (Variables|Default|GetTarget) (Math|Random|RandomRotator false)) "Undefined" 0 "0.000000,0.000000,0.000000" "0.000000,0.000000,0.000000" "0.000000,0.000000,0.000000")))

(fn ConstructionScript)