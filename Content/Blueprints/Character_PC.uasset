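; Player controller that routes movement and mouse-look axis input for the player's character.
; MoveForward and MoveRight cast the controlled pawn to Character on each axis event and pass the value to that character's matching movement function.
; Turn and LookUp feed yaw and pitch input straight into the controller's rotation.
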(event EventBeginPlay)

(event EventTick
  (params (DeltaSeconds :type Float%20%28single-precision%29)))

(event Input|AxisEvents|InputAxisMoveForward
  (params (AxisValue :type Float%20%28single-precision%29))
  ;[1 1 1] Movement
  (bind _ascharacter (Utilities|Casting|CastToCharacter (Pawn|GetControlledPawn)))
  (Default|MoveForward _ascharacter AxisValue))

(event Input|AxisEvents|InputAxisMoveRight
  (params (AxisValue :type Float%20%28single-precision%29))
  ;[1 1 1] Movement
  (bind _ascharacter (Utilities|Casting|CastToCharacter (Pawn|GetControlledPawn)))
  (Default|MoveRight _ascharacter AxisValue))

(event Input|AxisEvents|InputAxisTurn
  (params (AxisValue :type Float%20%28single-precision%29))
  ;[1 1 1] Mouse Rotation
  (Class|PlayerController|AddYawInput AxisValue))

(event Input|AxisEvents|InputAxisLookUp
  (params (AxisValue :type Float%20%28single-precision%29))
  ;[1 1 1] Mouse Rotation
  (Class|PlayerController|AddPitchInput AxisValue))

(fn ConstructionScript)