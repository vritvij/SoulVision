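; Flocking boid actor that steers itself with Reynolds-style rules inside a bounding box.
; Each tick it sphere-traces for neighbouring boids, then sums separation, alignment, cohesion and boundary forces, weighted by BoidManager.
; Update integrates the clamped velocity per frame, without delta time, and faces the boid along its movement.
; Seek, Arrive, Flee and a vision-cone test exist but are disconnected; the fetched player target goes unused.
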(event Custom|check)

(event EventTick
  (params (DeltaSeconds :type Float%20%28single-precision%29))
  (bind _boidmanager (Variables|Default|GetBoidManager))
  (Variables|Default|SetPosition (Transformation|GetActorLocation))
  (CallFunction|GetNeighbours (Variables|/Game/Boids/BoidManager.BoidManager_C|GetNeighbourhoodRadius (Variables|Default|GetBoidManager)))
  (bind _target (CallFunction|GetTarget))
  (bind _steeringforce (CallFunction|Separate))
  (bind _steeringforce_2 (CallFunction|Align))
  (bind _steeringforce_3 (CallFunction|Cohesion))
  (bind _steeringforce_4 (CallFunction|StayWithinBoundary))
  (CallFunction|ApplyForce (* _steeringforce (Variables|/Game/Boids/BoidManager.BoidManager_C|GetSeparation _boidmanager)))
  (CallFunction|ApplyForce (* _steeringforce_2 (Variables|/Game/Boids/BoidManager.BoidManager_C|GetAlignment _boidmanager)))
  (CallFunction|ApplyForce (* _steeringforce_3 (Variables|/Game/Boids/BoidManager.BoidManager_C|GetCohesion _boidmanager)))
  (CallFunction|ApplyForce (* _steeringforce_4 (Variables|/Game/Boids/BoidManager.BoidManager_C|GetStayWithinBounds _boidmanager)))
  (CallFunction|Update))

(fn ConstructionScript
  (Variables|Default|SetPosition (Transformation|GetActorLocation))
  (Variables|Default|SetVelocity (* (Transformation|GetActorForwardVector) 4)))

(fn GetTarget
  (bind _astest_pc (Utilities|Casting|CastToTest_PC (Game|GetPlayerController 0))
    (:then
      (return (Variables|/Game/Blueprints/Test_PC.Test_PC_C|GetTarget _astest_pc)))
    (:CastFailed
      (return "0, 0, 0"))))

(fn Seek
  (params (Target :type Vector))
  ;[1 1 1] Seek Behavior
  (return (Math|Vector|ClampVectorSize (- (* (Math|Vector|Normalize (- Target (Variables|Default|GetPosition))) (Variables|Default|GetMaxSpeed)) (Variables|Default|GetVelocity)) 0.0 (Variables|Default|GetMaxForce))))

(fn Arrive
  (params (Target :type Vector) (ArrivalRadius :type Float%20%28single-precision%29))
  (bind _position (Variables|Default|GetPosition))
  (bind _returnvalue (- Target _position))
  (bind _returnvalue_2 (Math|Vector|Normalize _returnvalue))
  (bind _returnvalue_3 (Math|Vector|VectorLength _returnvalue))
  ;[1 1 1] Arrival Behavior
  ;;[1 1 1] Check if distance to target is less than slow down radius
  (if (< _returnvalue_3 ArrivalRadius)
    (return (Math|Vector|ClampVectorSize (- (* _returnvalue_2 (Math|Float|MapRangeClamped _returnvalue_3 0.0 ArrivalRadius 0.0 (Variables|Default|GetMaxSpeed))) (Variables|Default|GetVelocity)) 0.0 (Variables|Default|GetMaxForce)))
    (else
      (return (Math|Vector|ClampVectorSize (- (* _returnvalue_2 (Variables|Default|GetMaxSpeed)) (Variables|Default|GetVelocity)) 0.0 (Variables|Default|GetMaxForce))))))

(fn StayWithinBoundary
  (bind _maxspeed (Variables|Default|GetMaxSpeed))
  (bind _returnvalue (* _maxspeed -1.0))
  (LocalVariables|SetDesiredVelocity (Variables|Default|GetVelocity))
  (Utilities|FlowControl|Sequence
    (:then_0
      (if (not (.IsInside? (CallFunction|DistancefromBoundary (Variables|Default|GetPosition) (Variables|Default|GetBoundBoxOrigin) (Variables|Default|GetBoundBoxExtent) (Variables|Default|GetBoundBoxRotation) "NewEnumerator0")))
        (LocalVariables|SetDesiredVelocity (Math|Vector|MakeVector _returnvalue (.Y (Math|Vector|BreakVector (LocalVariables|GetDesiredVelocity))) (.Z (Math|Vector|BreakVector (LocalVariables|GetDesiredVelocity)))))
        (elif (not (.IsInside? (CallFunction|DistancefromBoundary (Variables|Default|GetPosition) (Variables|Default|GetBoundBoxOrigin) (Variables|Default|GetBoundBoxExtent) (Variables|Default|GetBoundBoxRotation) "NewEnumerator1")))
          (LocalVariables|SetDesiredVelocity (Math|Vector|MakeVector _maxspeed (.Y (Math|Vector|BreakVector (LocalVariables|GetDesiredVelocity))) (.Z (Math|Vector|BreakVector (LocalVariables|GetDesiredVelocity))))))))
    (:then_1
      (if (not (.IsInside? (CallFunction|DistancefromBoundary (Variables|Default|GetPosition) (Variables|Default|GetBoundBoxOrigin) (Variables|Default|GetBoundBoxExtent) (Variables|Default|GetBoundBoxRotation) "NewEnumerator2")))
        (LocalVariables|SetDesiredVelocity (Math|Vector|MakeVector (.X (Math|Vector|BreakVector (LocalVariables|GetDesiredVelocity))) _returnvalue (.Z (Math|Vector|BreakVector (LocalVariables|GetDesiredVelocity)))))
        (elif (not (.IsInside? (CallFunction|DistancefromBoundary (Variables|Default|GetPosition) (Variables|Default|GetBoundBoxOrigin) (Variables|Default|GetBoundBoxExtent) (Variables|Default|GetBoundBoxRotation) "NewEnumerator3")))
          (LocalVariables|SetDesiredVelocity (Math|Vector|MakeVector (.X (Math|Vector|BreakVector (LocalVariables|GetDesiredVelocity))) _maxspeed (.Z (Math|Vector|BreakVector (LocalVariables|GetDesiredVelocity))))))))
    (:then_2
      (if (not (.IsInside? (CallFunction|DistancefromBoundary (Variables|Default|GetPosition) (Variables|Default|GetBoundBoxOrigin) (Variables|Default|GetBoundBoxExtent) (Variables|Default|GetBoundBoxRotation) "NewEnumerator4")))
        (LocalVariables|SetDesiredVelocity (Math|Vector|MakeVector (.X (Math|Vector|BreakVector (LocalVariables|GetDesiredVelocity))) (.Y (Math|Vector|BreakVector (LocalVariables|GetDesiredVelocity))) _returnvalue))
        (elif (not (.IsInside? (CallFunction|DistancefromBoundary (Variables|Default|GetPosition) (Variables|Default|GetBoundBoxOrigin) (Variables|Default|GetBoundBoxExtent) (Variables|Default|GetBoundBoxRotation) "NewEnumerator5")))
          (LocalVariables|SetDesiredVelocity (Math|Vector|MakeVector (.X (Math|Vector|BreakVector (LocalVariables|GetDesiredVelocity))) (.Y (Math|Vector|BreakVector (LocalVariables|GetDesiredVelocity))) _maxspeed)))))
    (:then_3
      (return (Math|Vector|ClampVectorSize (- (* (Math|Vector|Normalize (LocalVariables|GetDesiredVelocity)) (Variables|Default|GetMaxSpeed)) (Variables|Default|GetVelocity)) 0.0 (Variables|Default|GetMaxForce))))))

(fn ApplyForce
  (params (Force :type Vector))
  (Variables|Default|SetAcceleration (+ Force (Variables|Default|GetAcceleration))))

(fn Update
  ;[1 1 1] Update boid position and rotation
  ;;[1 1 1] Calculate new velocity
  (bind _output_get (Variables|Default|SetVelocity (Math|Vector|ClampVectorSize (+ (Variables|Default|GetVelocity) (Variables|Default|GetAcceleration)) 0.0 (Variables|Default|GetMaxSpeed))))
  ;;[1 1 1] Calculate boid's new position
  (bind _output_get_2 (Variables|Default|SetPosition (+ _output_get (Variables|Default|GetPosition))))
  (Transformation|SetActorLocationAndRotation _output_get_2 (Math|Rotator|FindLookatRotation (Transformation|GetActorLocation) (Variables|Default|GetPosition)))
  ;;[1 1 1] Reset acceleration
  (Variables|Default|SetAcceleration "0, 0, 0"))

(fn Align
  (bind _neighbours (Variables|Default|GetNeighbours))
  (for _array_element _neighbours
    (LocalVariables|SetAverageVelocity (+ (Variables|Boid_BP_C|GetVelocity _array_element) (LocalVariables|GetAverageVelocity))))
  (return (Math|Vector|ClampVectorSize (- (* (Math|Vector|Normalize (+ (/ (LocalVariables|GetAverageVelocity) (Utilities|Array|Length _neighbours)) (Variables|Default|GetVelocity))) (Variables|Default|GetMaxSpeed)) (Variables|Default|GetVelocity)) 0.0 (Variables|Default|GetMaxForce))))

(fn GetNeighbours
  (params (NeighbourhoodRadius :type Float%20%28single-precision%29))
  (bind _position (Variables|Default|GetPosition))
  (Utilities|Array|Clear (Variables|Default|GetNeighbours))
  (bind _outhits (Collision|MultiSphereTraceForObjects _position (+ _position "0, 0,0.100000") NeighbourhoodRadius (Utilities|Array|MakeArray "ObjectTypeQuery2") false 0 "None"))
  (for _array_element _outhits
    (bind _asboid_bp (Utilities|Casting|CastToBoid_BP (.HitActor (Collision|BreakHitResult _array_element))))
    (Utilities|Array|Add (Variables|Default|GetNeighbours) _asboid_bp)))

(fn Flee
  (params (Target :type Vector))
  ;[1 1 1] Seek Behavior
  (return (Math|Vector|ClampVectorSize (- (Math|Vector|NegateVector (* (Math|Vector|Normalize (- Target (Variables|Default|GetPosition))) (Variables|Default|GetMaxSpeed))) (Variables|Default|GetVelocity)) 0.0 (Variables|Default|GetMaxForce))))

(fn Separate
  (bind _neighbours (Variables|Default|GetNeighbours))
  (bind _returnvalue (Utilities|Array|Length _neighbours))
  (for _array_element _neighbours
    (LocalVariables|SetAverageSeparation (+ (/ (Math|Vector|Normalize (- (Variables|Default|GetPosition) (Variables|Boid_BP_C|GetPosition _array_element))) (Math|Vector|VectorLength (- (Variables|Default|GetPosition) (Variables|Boid_BP_C|GetPosition _array_element)))) (LocalVariables|GetAverageSeparation))))
  (if (> _returnvalue 0)
    (return (Math|Vector|ClampVectorSize (- (* (Math|Vector|Normalize (/ (LocalVariables|GetAverageSeparation) _returnvalue)) (Variables|Default|GetMaxSpeed)) (Variables|Default|GetVelocity)) 0.0 (Variables|Default|GetMaxForce)))
    (else
      (return "0, 0, 0"))))

(fn Cohesion
  (bind _neighbours (Variables|Default|GetNeighbours))
  (for _array_element _neighbours
    (LocalVariables|SetCenterOfMass (+ (Variables|Boid_BP_C|GetPosition _array_element) (LocalVariables|GetCenterOfMass))))
  (return (Math|Vector|ClampVectorSize (- (* (Math|Vector|Normalize (+ (/ (LocalVariables|GetCenterOfMass) (Utilities|Array|Length _neighbours)) (Variables|Default|GetVelocity))) (Variables|Default|GetMaxSpeed)) (Variables|Default|GetVelocity)) 0.0 (Variables|Default|GetMaxForce))))